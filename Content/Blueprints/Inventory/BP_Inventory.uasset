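; BP_Inventory stores the player's items in a fixed-size slot array and toggles the inventory menu.
; On BeginPlay it sizes the array to ItemSpace, and AddInventory writes non-stackable items into the first empty slot, with no handling for stackable ones.
; OpenClose creates or removes the menu widget, centre-anchored on the TopDownController's HUD canvas, switching between UI-only and game-only input.
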(event `self.ReceiveBeginPlay`
  (`self.StartInventory`))

(fn `Add Inventory`
  (params (ContentToAdd :type "/Game/Blueprints/Inventory/STR_ItemSpace Structure"))
  (returns (`Add?` :type Boolean))
  (if (not (`.EsStackUp_11_8DDC558F48D5CAB86695048B2252E8D8` (break `/Game/Blueprints/Inventory/STR_Item` (break `/Game/Blueprints/Inventory/STR_ItemSpace` ContentToAdd))))
    (`self.CreatePilha` (`local.ContentToAdd`))
    (return true)))

(fn `CreatePilha`
  (params (ContentAdd :type "/Game/Blueprints/Inventory/STR_ItemSpace Structure"))
  (bind _iventory (`self.Iventory`))
  (`KismetArrayLibrary.Array_Set` _iventory (`KismetArrayLibrary.Array_Find` _iventory (make `/Game/Blueprints/Inventory/STR_ItemSpace` (struct :`nAME` "NSLOCTEXT(\"[B63951554ACC1535DA20AB9D05CB1242]\", \"4F383C754A9D97B7BA8AB1B64C91123C\", \"NONE\")" :`EsStackUp` true :`MaxStackUp` 5))) ContentAdd))

(fn `OpenClose`
  (bind _windowmenuinventory (`self.WindowMenuInventory`))
  (bind _windowmenuinventory_2 (`self.WindowMenuInventory`)
    (:`then`
      (`Widget.RemoveFromParent` _windowmenuinventory_2)
      (set `self.WindowMenuInventory` null)
      (`WidgetBlueprintLibrary.SetInputMode_GameOnly` (`GameplayStatics.GetPlayerController` 0)))
    (:`else`
      (bind _returnvalue (`|CreateWidget` "/Game/Blueprints/Widget/HUD_MenuInventory.HUD_MenuInventory_C" (`GameplayStatics.GetPlayerController` 0) self))
      (set `self.WindowMenuInventory` _returnvalue)
      (bind _astop_down_controller (cast `/Game/TopDownBP/Blueprints/TopDownController` (`GameplayStatics.GetPlayerController` 0)))
      (bind _returnvalue_2 (`CanvasPanel.AddChildToCanvas` (`/Game/Blueprints/Widget/HUD_Player.HUDPlayer` (`/Game/TopDownBP/Blueprints/TopDownController.HudScreen` _astop_down_controller)) _windowmenuinventory))
      (`CanvasPanelSlot.SetAutoSize` _returnvalue_2 true)
      (`CanvasPanelSlot.SetAlignment` _returnvalue_2 (0.5 0.5))
      (`CanvasPanelSlot.SetAnchors` _returnvalue_2 (make `Anchors` (0.5 0.5) (0.5 0.5)))
      (`CanvasPanelSlot.SetPosition` _returnvalue_2 (`self.Position`))
      (`WidgetBlueprintLibrary.SetInputMode_UIOnlyEx` (`GameplayStatics.GetPlayerController` 0) _windowmenuinventory "LockAlways"))))

(fn `StartInventory`
  (`KismetArrayLibrary.Array_Resize` (`self.Iventory`) (`self.ItemSpace`)))