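; Interactive hand sanitizer item (álcool gel dispenser) that ends the level when collected.
; Any actor overlap enables player input and opens a Gate, which is never closed, for the E key.
; Pressing E destroys the four dispenser meshes, plays a coin sound and loads "Victory", or "Defeal" if the actor is being destroyed.
; Only components are destroyed, so the check normally leads to "Victory".
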(event `Key|E`
  (params (Key :type "Key Structure"))
  (:`Pressed`
    (`/Engine/EditorBlueprintResources/StandardMacros.Gate` true :!label _label
      (:`Exit`
        (`ActorComponent.K2_DestroyComponent` (`self.uploads_files_2564844_Soap+Dispenser_Cylinder_003`))
        (`ActorComponent.K2_DestroyComponent` (`self.uploads_files_2564844_Soap+Dispenser_Cylinder_001`))
        (`ActorComponent.K2_DestroyComponent` (`self.uploads_files_2564844_Soap+Dispenser_Cylinder_002`))
        (`ActorComponent.K2_DestroyComponent` (`self.uploads_files_2564844_Soap+Dispenser_Cylinder`))
        (`GameplayStatics.PlaySound2D` "/Game/Assets/Sounds/Coin_Collect_sound_effect__online-audio-converter_com_.Coin_Collect_sound_effect__online-audio-converter_com_" 1.0 1.0 0.0 null null)
        (if (`self.IsActorBeingDestroyed`)
          (`GameplayStatics.OpenLevel` "Defeal")
          (else
            (`GameplayStatics.OpenLevel` "Victory")))))))

(event `self.ReceiveActorBeginOverlap`
  (params (OtherActor :type "Actor Object Reference"))
  (`self.EnableInput` (`GameplayStatics.GetPlayerController` 0))
  (goto _label :!via `Open`))

(fn `UserConstructionScript`)