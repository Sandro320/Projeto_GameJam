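; BP_Mask is an interactable mask item that is collected with the E key.
; Actor overlap enables player input and opens a Gate, which nothing closes because end overlap is empty.
; E then drives a FlipFlop: the first press destroys both mask meshes and plays a coin sound, while the next tries to unhide those components.
; A CreateWidget node is left unconnected.
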(event `Key|E`
  (params (Key :type "Key Structure"))
  (bind _mask_fbx_mask (`self.Mask_FBX_Mask`))
  (:`Pressed`
    (`/Engine/EditorBlueprintResources/StandardMacros.Gate` true :!label _label
      (:`Exit`
        (`/Engine/EditorBlueprintResources/StandardMacros.FlipFlop`
          (:`A`
            (`ActorComponent.K2_DestroyComponent` _mask_fbx_mask)
            (`ActorComponent.K2_DestroyComponent` (`self.Mask_FBX_1`))
            (`GameplayStatics.PlaySound2D` "/Game/Assets/Sounds/Coin_Collect_sound_effect__online-audio-converter_com_.Coin_Collect_sound_effect__online-audio-converter_com_" 1.0 1.0 0.0 null null))
          (:`B`
            (`SceneComponent.SetHiddenInGame` _mask_fbx_mask false false)
            (`SceneComponent.SetHiddenInGame` (`self.Mask_FBX_1`) false false)))))))

(event `self.ReceiveActorBeginOverlap`
  (params (OtherActor :type "Actor Object Reference"))
  (`self.EnableInput` (`GameplayStatics.GetPlayerController` 0))
  (goto _label :!via `Open`))

(event `self.Box.OnComponentEndOverlap`
  (params (OverlappedComponent :type "PrimitiveComponent Object Reference") (OtherActor :type "Actor Object Reference") (OtherComp :type "PrimitiveComponent Object Reference") (OtherBodyIndex :type Integer)))

(fn `UserConstructionScript`)