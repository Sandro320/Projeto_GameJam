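; Item actor that infects on contact and starts a timed countdown to defeat.
; Any overlap with its Box shows the Infectado widget, sets a play rate from the inverse of TimeToDie and plays the Countdown timeline.
; The timeline writes its truncated Time value back into TimeToDie each update.
; When it finishes, the game pauses and the Defeal widget appears.
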(event `self.Box.OnComponentBeginOverlap`
  (params (OverlappedComponent :type "PrimitiveComponent Object Reference") (OtherActor :type "Actor Object Reference") (OtherComp :type "PrimitiveComponent Object Reference") (OtherBodyIndex :type Integer) (bFromSweep :type Boolean) (SweepResult :type "HitResult Structure (by ref)"))
  (bind _returnvalue (`|CreateWidget` "/Game/Blueprints/Widget/Infectado.Infectado_C"))
  (`UserWidget.AddToViewport` _returnvalue 0)
  (`MovieSceneSequencePlayer.SetPlayRate` (`self.Time`) (/ 1.0 (`KismetSystemLibrary.MakeLiteralDouble` (`KismetMathLibrary.Conv_IntToDouble` (`self.TimeToDie`)))))
  (bind (_direction _time) (`Timeline|Countdown`)
    (:`Update`
      (set `self.TimeToDie` (`KismetMathLibrary.FTrunc` _time)))
    (:`Finished`
      (`GameplayStatics.SetGamePaused` true)
      (bind _returnvalue_2 (`|CreateWidget` "/Game/Blueprints/Widget/Defeal.Defeal_C"))
      (`UserWidget.AddToViewport` _returnvalue_2 0))))

(fn `UserConstructionScript`)